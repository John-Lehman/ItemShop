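; Base paper-flipbook pawn that can carry objects through pickup messages and can itself be picked up by another character.
; Pickup disables capsule collision, then a Tick-driven state machine lerps actor and sprite separately toward the carrier, using attach and offset sockets, before attaching both.
; Being dropped or thrown is stubbed out.
; Overlaps with NavModifierVolumes of the InsideShop area class track whether it is inside the shop.
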(event Custom|OnPawnBeginOverlapEvent
  (params (OverlappedActor :type Actor%20Object%20Reference) (OtherActor :type Actor%20Object%20Reference))
  (bind _asnav_modifier_volume (Utilities|Casting|CastToNavModifierVolume OtherActor))
  (if (== (Variables|/Script/Engine.NavModifierVolume|GetAreaClass _asnav_modifier_volume) "/Game/Blueprints/Shop/NAVAREA_InsideShop.NAVAREA_InsideShop_C")
    (Utilities|Array|Add (Variables|NavAreas|GetOverlappingNavAreas) _asnav_modifier_volume)))

(event Custom|OnPawnEndOverlapEvent
  (params (OverlappedActor :type Actor%20Object%20Reference) (OtherActor :type Actor%20Object%20Reference))
  (bind _asnav_modifier_volume (Utilities|Casting|CastToNavModifierVolume OtherActor))
  (if (== (Variables|/Script/Engine.NavModifierVolume|GetAreaClass _asnav_modifier_volume) "/Game/Blueprints/Shop/NAVAREA_InsideShop.NAVAREA_InsideShop_C")
    (Utilities|Array|RemoveItem (Variables|NavAreas|GetOverlappingNavAreas) _asnav_modifier_volume)))

(event EventBeginPlay
  (Collision|BindEventtoOnActorBeginOverlap (delegate Custom|OnPawnBeginOverlapEvent))
  (Collision|BindEventtoOnActorEndOverlap (delegate Custom|OnPawnEndOverlapEvent)))

(event EventTick
  (params (DeltaSeconds :type Float%20%28single-precision%29))
  (Update|UpdatePickup))

(fn ConstructionScript)

(fn CanPickupAnything
  (return (not (Utilities|IsValid (Variables|PickupCharacter|GetHeldObject)))))

(fn CanThrowActor
  (if (Utilities|IsValid (Variables|PickupCharacter|GetHeldObject))
    (bind _result (Class|INTERFPickupActor|CanbeThrown(Message) (Variables|PickupCharacter|GetHeldObject)))
    (return _result)
    (else
      (return false))))

(fn CanDropActor
  (if (Utilities|IsValid (Variables|PickupCharacter|GetHeldObject))
    (bind _results (Class|INTERFPickupActor|CanbeDropped(Message) (Variables|PickupCharacter|GetHeldObject)))
    (return _results)
    (else
      (return false))))

(fn TryPickup
  (params (Target :type Actor%20Object%20Reference) (Direction :type Vector))
  (LocalVariables|SetHitActor Target)
  (LocalVariables|SetPickupDirection Direction)
  (if (Pickup|CanPickupAnything)
    (if (Utilities|IsValid (LocalVariables|GetHitActor))
      (bind _results (Class|INTERFPickupActor|CanbePickedUp(Message) (LocalVariables|GetHitActor)))
      (if _results
        (Class|INTERFPickupActor|BecomePickedUp(Message) (LocalVariables|GetHitActor) self)
        (Variables|PickupCharacter|SetHeldObject (LocalVariables|GetHitActor))))
    (else
      (bind _results_2 (Class|INTERFPickupActor|CanbeDropped(Message) (Variables|PickupCharacter|GetHeldObject)))
      (if _results_2
        (Class|INTERFPickupActor|BecomeDropped(Message) (Variables|PickupCharacter|GetHeldObject))
        (Variables|PickupCharacter|SetHeldObject 0)))))

(fn RemoveHeldObject
  (Variables|PickupCharacter|SetHeldObject 0))

(fn IsInsideShop
  (return (> (Utilities|Array|Length (Variables|NavAreas|GetOverlappingNavAreas)) 0)))

(fn UpdatePickup
  (switch Utilities|FlowControl|Switch|SwitchonENUM_PickupState (.transition_state (Variables|PickupCharacter|GetPickupData))
    (:NewEnumerator1
      (Update|UpdateMounting))
    (:NewEnumerator2
      (Update|UpdateDismounting))
    (:NewEnumerator4
      (Update|UpdateThrown))))

(fn UpdateMounting
  (bind _shopgameinstance (Utilities|GetShopGameInstance))
  (bind _pickupdata (Variables|PickupCharacter|GetPickupData))
  (bind _pickupdata_2 (Variables|PickupCharacter|GetPickupData))
  (bind _socketnames (Variables|/Game/Blueprints/GAME_ShopGame.GAME_ShopGame_C|GetSocketNames _shopgameinstance))
  (LocalVariables|SetProgress (Math|Float|Clamp(Float) (/ (- (Utilities|Time|GetGameTimeinSeconds) (.transition_starttimestamp _pickupdata)) (Utilities|Select :Index (.transition_state _pickupdata) :NewEnumerator0 0.0 :NewEnumerator1 (.preset_mountduration _pickupdata) :NewEnumerator2 (.preset_dismountduration _pickupdata) :NewEnumerator3 0.0 :NewEnumerator4 0.0))))
  (LocalVariables|SetStartLocation_Actor (.transition_startlocation _pickupdata_2))
  (LocalVariables|SetEndLocation_Actor (Transformation|GetActorLocation (.attach_character _pickupdata_2)))
  (LocalVariables|SetPickupAttachName (.pickup_attach _socketnames))
  (LocalVariables|SetPickupOffsetName (.pickup_offset _socketnames))
  (LocalVariables|SetStartLocation_Sprite (.attach_startlocation (Variables|PickupCharacter|GetPickupData)))
  (Utilities|FlowControl|Sequence
    (:then_0
      (if (Transformation|DoesSocketExist (Variables|PAWN_PickupCharacter_C|GetPaperFlipbook (.attach_character (Variables|PickupCharacter|GetPickupData))) (LocalVariables|GetPickupAttachName))
        (LocalVariables|SetEndLocation_Sprite (Transformation|GetSocketLocation (Variables|PAWN_PickupCharacter_C|GetPaperFlipbook (.attach_character (Variables|PickupCharacter|GetPickupData))) (LocalVariables|GetPickupAttachName)))
        (else
          (LocalVariables|SetEndLocation_Sprite (LocalVariables|GetEndLocation_Actor)))))
    (:then_1
      (if (Transformation|DoesSocketExist (Variables|Default|GetPaperFlipbook) (LocalVariables|GetPickupOffsetName))
        (LocalVariables|SetEndLocation_Sprite (+ (LocalVariables|GetEndLocation_Sprite) (- (Transformation|GetWorldLocation (Variables|Default|GetPaperFlipbook)) (Transformation|GetSocketLocation (Variables|Default|GetPaperFlipbook) (LocalVariables|GetPickupOffsetName)))))))
    (:then_2
      (Transformation|SetWorldLocation (Variables|Default|GetPaperFlipbook) (Math|Vector|Lerp(Vector) (LocalVariables|GetStartLocation_Sprite) (LocalVariables|GetEndLocation_Sprite) (LocalVariables|GetProgress)) false false)
      (Transformation|SetActorLocation (Math|Vector|Lerp(Vector) (LocalVariables|GetStartLocation_Actor) (LocalVariables|GetEndLocation_Actor) (LocalVariables|GetProgress)) false false))
    (:then_3
      (if (== (LocalVariables|GetProgress) 1.0)
        (Utilities|Struct|SetmembersinSTRUCT_PickupData (Variables|PickupCharacter|GetPickupData) "NewEnumerator3")
        (Transformation|AttachActorToActor (.attach_character (Variables|PickupCharacter|GetPickupData)) "None" "SnapToTarget" "KeepWorld" "KeepWorld" false)
        (Transformation|AttachComponentToComponent (Variables|Default|GetPaperFlipbook) (Variables|PAWN_PickupCharacter_C|GetPaperFlipbook (.attach_character (Variables|PickupCharacter|GetPickupData))) (select (Transformation|DoesSocketExist (Variables|Default|GetPaperFlipbook) (LocalVariables|GetPickupAttachName)) (LocalVariables|GetPickupAttachName) "None") "KeepWorld" "KeepWorld" "KeepWorld" false)))))

(fn UpdateDismounting)

(fn UpdateThrown)

(fn BecomeDropped
  (return false))

(fn BecomePickedUp
  (params (PickupCharacter :type PAWN%20Pickup%20Character%20Object%20Reference))
  (Utilities|Struct|SetmembersinSTRUCT_PickupData (Variables|PickupCharacter|GetPickupData) "NewEnumerator1" (Utilities|Time|GetGameTimeinSeconds) (Transformation|GetActorLocation) PickupCharacter (Transformation|GetWorldLocation (Variables|Default|GetPaperFlipbook)) (Variables|/Script/Engine.SceneComponent|GetRelativeLocation (Variables|Default|GetPaperFlipbook)))
  (Collision|SetCollisionEnabled (Variables|Collision|GetCapsuleComponent) "NoCollision")
  (return true))

(fn BecomeThrown
  (return false))

(fn CanbeDropped
  (return false))

(fn CanbePickedUp
  (return (Utilities|Enum|Equal(Enum) (.transition_state (Variables|PickupCharacter|GetPickupData)) "NewEnumerator0")))

(fn CanbeThrown
  (return false))

(fn GetPickupState
  (return (.transition_state (Variables|PickupCharacter|GetPickupData))))