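; Blueprint interface for item shop actors that a character can pick up, throw or drop.
; It pairs query functions for whether each action is allowed with functions that perform the action, with the picking character passed in on pickup.
; A further getter exposes the actor's pickup state as an enum, and the interface holds no logic of its own, leaving behavior to implementers.
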(fn CanbePickedUp
  (return false))

(fn BecomePickedUp
  (params (PickupCharacter :type PAWN%20Pickup%20Character%20Object%20Reference))
  (return false))

(fn BecomeThrown
  (return false))

(fn BecomeDropped
  (return false))

(fn CanbeThrown
  (return false))

(fn CanbeDropped
  (return false))

(fn GetPickupState
  (return "NewEnumerator0"))