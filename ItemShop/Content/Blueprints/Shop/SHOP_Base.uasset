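; SHOP_Base is a shop Blueprint that keeps a registry of item display containers and hands one out on request.
; Containers are registered once each through RegisterDisplayContainer.
; GetItemDisplayContainer gathers those whose IsAtCapacity check returns true into FreeDisplays, despite that name, and returns a random entry, or nothing when that list is empty.
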(fn ConstructionScript)

(fn RegisterDisplayContainer
  (params (DisplayContainer :type CONTAINER%20Display%20Object%20Reference))
  (Utilities|Array|AddUnique (Variables|ItemDisplay|GetDisplayContainers) DisplayContainer))

(fn GetItemDisplayContainer
  (for _array_element (Variables|ItemDisplay|GetDisplayContainers)
    (if (Default|IsatCapacity _array_element)
      (Utilities|Array|Add (LocalVariables|GetFreeDisplays) _array_element)))
  (if (> (Utilities|Array|Length (LocalVariables|GetFreeDisplays)) 0)
    (return (Utilities|Array|Get(acopy) (LocalVariables|GetFreeDisplays) (Math|Random|RandomIntegerinRange 0 (Utilities|Array|LastIndex (LocalVariables|GetFreeDisplays)))))
    (else
      (return 0))))