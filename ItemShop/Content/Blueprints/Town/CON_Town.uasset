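; CON_Town is a controller that runs the BT_Town behavior tree and manages the town's population of PAWN_Customer citizens.
; On BeginPlay it caches all VOLUME_Spawner actors, then starts the tree.
; SpawnCitizen picks a random spawner and point, spawns a customer with randomized Stamina, then records it in ActiveCitizens with a timestamp.
; DespawnCitizen only removes the citizen from that list, without destroying the actor.
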(event EventBeginPlay
  (bind _outactors (Actor|GetAllActorsOfClass "/Game/Blueprints/Volumes/VOLUME_Spawner.VOLUME_Spawner_C"))
  (Variables|Citizens|SetSpawners _outactors)
  (AI|RunBehaviorTree "/Game/Blueprints/Town/Behaviors/BT_Town.BT_Town"))

(fn ConstructionScript)

(fn SpawnCitizen
  (if (> (Utilities|Array|Length (Variables|Citizens|GetSpawners)) 0)
    (LocalVariables|SetSpawnerToUse (Utilities|Array|Get(acopy) (Variables|Citizens|GetSpawners) (Math|Random|RandomInteger (Utilities|Array|Length (Variables|Citizens|GetSpawners)))))
    (LocalVariables|SetSpawnLocation (+ (Math|Vector|MakeVector (.x (Default|GetRandomPointinBox (LocalVariables|GetSpawnerToUse))) (.y (Default|GetRandomPointinBox (LocalVariables|GetSpawnerToUse))) 0.0) "0.000000, 0,15.000000"))
    (bind _returnvalue (Game|SpawnActorfromClass "/Game/Blueprints/PickupCharacters/Citizen/PAWN_Customer.PAWN_Customer_C" (Math|Transform|MakeTransform (LocalVariables|GetSpawnLocation) "0, 0, 0" "1,1,1") "AdjustIfPossibleButDontSpawnIfColliding" 0 (LocalVariables|GetSpawnerToUse) (Math|Random|RandomIntegerinRange 0 1)))
    (if (Utilities|IsValid _returnvalue)
      (Utilities|Array|Add (Variables|Citizens|GetActiveCitizens) _returnvalue)
      (Variables|Citizens|SetSpawnCitizen_Timestamp (Utilities|Time|GetGameTimeinSeconds)))
    (else
      (Development|PrintString "Can't spawn customer because no spawner detected at startup." false))))

(fn DespawnCitizen
  (params (Citizen :type PAWN%20Customer%20Object%20Reference))
  (bind _returnvalue (Utilities|Array|RemoveItem (Variables|Citizens|GetActiveCitizens) Citizen))
  (return _returnvalue))