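; Base pickup actor with a Paper2D sprite that characters can pick up, carry and drop.
; Tick runs a transition state machine that lerps actor and sprite separately over timed mount and dismount durations.
; Mounting aligns the sprite to character flipbook sockets, then attaches it; dropping detaches toward the character's facing and restores box collision afterward.
; Throwing is stubbed, and GetPickupState always returns Free.
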(event EventTick
  (params (DeltaSeconds :type Float%20%28single-precision%29))
  (Update|UpdatePickup))

(fn ConstructionScript)

(fn UpdatePickup
  (switch Utilities|FlowControl|Switch|SwitchonENUM_PickupState (.transition_state (Variables|PickupObject|GetPickupData))
    (:NewEnumerator1
      (Update|UpdateMounting))
    (:NewEnumerator2
      (Update|UpdateDismounting))
    (:NewEnumerator4
      (Update|UpdateThrown))))

(fn UpdateMounting
  (bind _shopgameinstance (Utilities|GetShopGameInstance))
  (bind _pickupdata (Variables|PickupObject|GetPickupData))
  (bind _pickupdata_2 (Variables|PickupObject|GetPickupData))
  (bind _socketnames (Variables|/Game/Blueprints/GAME_ShopGame.GAME_ShopGame_C|GetSocketNames _shopgameinstance))
  (LocalVariables|SetProgress (Math|Float|Clamp(Float) (/ (- (Utilities|Time|GetGameTimeinSeconds) (.transition_starttimestamp _pickupdata)) (Utilities|Select :Index (.transition_state _pickupdata) :NewEnumerator0 0.0 :NewEnumerator1 (.preset_mountduration _pickupdata) :NewEnumerator2 (.preset_dismountduration _pickupdata) :NewEnumerator3 0.0 :NewEnumerator4 0.0))))
  (LocalVariables|SetStartLocation_Actor (.transition_startlocation _pickupdata_2))
  (LocalVariables|SetEndLocation_Actor (Transformation|GetActorLocation (.attach_character _pickupdata_2)))
  (LocalVariables|SetPickupAttachName (.pickup_attach _socketnames))
  (LocalVariables|SetPickupOffsetName (.pickup_offset _socketnames))
  (LocalVariables|SetStartLocation_Sprite (.attach_startlocation (Variables|PickupObject|GetPickupData)))
  (Utilities|FlowControl|Sequence
    (:then_0
      (if (Transformation|DoesSocketExist (Variables|/Game/Blueprints/PickupCharacters/PAWN_PickupCharacter.PAWN_PickupCharacter_C|GetPaperFlipbook (.attach_character (Variables|PickupObject|GetPickupData))) (LocalVariables|GetPickupAttachName))
        (LocalVariables|SetEndLocation_Sprite (Transformation|GetSocketLocation (Variables|/Game/Blueprints/PickupCharacters/PAWN_PickupCharacter.PAWN_PickupCharacter_C|GetPaperFlipbook (.attach_character (Variables|PickupObject|GetPickupData))) (LocalVariables|GetPickupAttachName)))
        (else
          (LocalVariables|SetEndLocation_Sprite (LocalVariables|GetEndLocation_Actor)))))
    (:then_1
      (if (Transformation|DoesSocketExist (Variables|Default|GetPaperSprite) (LocalVariables|GetPickupOffsetName))
        (LocalVariables|SetEndLocation_Sprite (+ (LocalVariables|GetEndLocation_Sprite) (- (Transformation|GetWorldLocation (Variables|Default|GetPaperSprite)) (Transformation|GetSocketLocation (Variables|Default|GetPaperSprite) (LocalVariables|GetPickupOffsetName)))))))
    (:then_2
      (Transformation|SetWorldLocation (Variables|Default|GetPaperSprite) (Math|Vector|Lerp(Vector) (LocalVariables|GetStartLocation_Sprite) (LocalVariables|GetEndLocation_Sprite) (LocalVariables|GetProgress)) false false)
      (Transformation|SetActorLocation (Math|Vector|Lerp(Vector) (LocalVariables|GetStartLocation_Actor) (LocalVariables|GetEndLocation_Actor) (LocalVariables|GetProgress)) false false))
    (:then_3
      (if (== (LocalVariables|GetProgress) 1.0)
        (Utilities|Struct|SetmembersinSTRUCT_PickupData (Variables|PickupObject|GetPickupData) "NewEnumerator3")
        (Transformation|AttachActorToActor (.attach_character (Variables|PickupObject|GetPickupData)) "None" "SnapToTarget" "KeepWorld" "KeepWorld" false)
        (Transformation|AttachComponentToComponent (Variables|Default|GetPaperSprite) (Variables|/Game/Blueprints/PickupCharacters/PAWN_PickupCharacter.PAWN_PickupCharacter_C|GetPaperFlipbook (.attach_character (Variables|PickupObject|GetPickupData))) (select (Transformation|DoesSocketExist (Variables|Default|GetPaperSprite) (LocalVariables|GetPickupAttachName)) (LocalVariables|GetPickupAttachName) "None") "KeepWorld" "KeepWorld" "KeepWorld" false)))))

(fn UpdateDismounting
  (bind _pickupdata (Variables|PickupObject|GetPickupData))
  (bind _pickupdata_2 (Variables|PickupObject|GetPickupData))
  (bind _pickupdata_3 (Variables|PickupObject|GetPickupData))
  (LocalVariables|SetProgress (Math|Float|Clamp(Float) (/ (- (Utilities|Time|GetGameTimeinSeconds) (.transition_starttimestamp _pickupdata)) (.preset_dismountduration _pickupdata))))
  (Transformation|SetActorLocation (Math|Vector|Lerp(Vector) (.transition_startlocation _pickupdata_2) (.transition_endlocation _pickupdata_2) (LocalVariables|GetProgress)) false false)
  (Transformation|SetWorldLocation (Variables|Default|GetPaperSprite) (Math|Vector|Lerp(Vector) (.attach_startlocation _pickupdata_3) (+ (.transition_endlocation _pickupdata_3) (.attach_relativelocation _pickupdata_3)) (LocalVariables|GetProgress)) false false)
  (if (== (LocalVariables|GetProgress) 1.0)
    (Utilities|Struct|SetmembersinSTRUCT_PickupData (Variables|PickupObject|GetPickupData) "NewEnumerator0")
    (Collision|SetCollisionEnabled (Variables|Default|GetBox) "QueryAndPhysics")))

(fn UpdateThrown)

(fn BecomeDropped
  (|GetForwardDirection
    (:out
      (LocalVariables|SetEndLocation (+ (Transformation|GetActorLocation) (* (LocalVariables|GetForwardDirection) 18.0)))
      (Utilities|Struct|SetmembersinSTRUCT_PickupData (Variables|PickupObject|GetPickupData) "NewEnumerator2" (Utilities|Time|GetGameTimeinSeconds) (Transformation|GetActorLocation) (LocalVariables|GetEndLocation) (Transformation|GetWorldLocation (Variables|Default|GetPaperSprite)))
      (Transformation|AttachComponentToComponent (Variables|Default|GetPaperSprite) (Variables|Default|GetBox) "None" "KeepWorld" "KeepWorld" "KeepWorld" false)
      (Transformation|DetachFromActor "KeepWorld" "KeepWorld" "KeepWorld")
      (return false))))

(fn BecomePickedUp
  (params (PickupCharacter :type PAWN%20Pickup%20Character%20Object%20Reference))
  (Utilities|Struct|SetmembersinSTRUCT_PickupData (Variables|PickupObject|GetPickupData) "NewEnumerator1" (Utilities|Time|GetGameTimeinSeconds) (Transformation|GetActorLocation) PickupCharacter (Transformation|GetWorldLocation (Variables|Default|GetPaperSprite)) (Variables|/Script/Engine.SceneComponent|GetRelativeLocation (Variables|Default|GetPaperSprite)))
  (Actor|Tick|SetActorTickEnabled true)
  (Collision|SetCollisionEnabled (Variables|Default|GetBox) "NoCollision")
  (return true))

(fn BecomeThrown
  (return false))

(fn CanbeDropped
  (return (Utilities|Enum|Equal(Enum) (.transition_state (Variables|PickupObject|GetPickupData)) "NewEnumerator3")))

(fn CanbePickedUp
  (return (Utilities|Enum|Equal(Enum) (.transition_state (Variables|PickupObject|GetPickupData)) "NewEnumerator0")))

(fn CanbeThrown
  (return (Utilities|Enum|Equal(Enum) (.transition_state (Variables|PickupObject|GetPickupData)) "NewEnumerator3")))

(fn GetPickupState
  (return "NewEnumerator0"))