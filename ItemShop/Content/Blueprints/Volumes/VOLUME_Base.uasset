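; VOLUME_Base is a base volume Blueprint built around a Box component.
; GetRandomPointInBox returns the box's world location plus a random offset within its scaled extent on each axis.
; The offset is not rotated, so the sampled region stays world-axis-aligned even if the box is rotated.
; The event graph and construction script hold no logic.
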(event EventBeginPlay)

(event Collision|EventActorBeginOverlap
  (params (OtherActor :type Actor%20Object%20Reference)))

(event EventTick
  (params (DeltaSeconds :type Float%20%28single-precision%29)))

(fn ConstructionScript)

(fn GetRandomPointinBox
  (bind _box (Variables|Default|GetBox))
  (bind _returnvalue (Components|Box|GetScaledBoxExtent _box))
  (return (+ (Transformation|GetWorldLocation (Variables|Default|GetBox)) (Math|Vector|MakeVector (Math|Random|RandomFloatinRange (* (.x _returnvalue) -1.0) (.x _returnvalue)) (Math|Random|RandomFloatinRange (* (.y _returnvalue) -1.0) (.y _returnvalue)) (Math|Random|RandomFloatinRange (* (.z _returnvalue) -1.0) (.z _returnvalue))))))