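; Blueprint utility of constant-acceleration kinematics helpers.
; GetTimeUntilVelocityIsReached divides the velocity change by acceleration, but prints a warning and returns a huge sentinel time when the target velocity is unreachable.
; GetDistanceAfterAcceleration returns displacement from start velocity, time and acceleration using the standard kinematic equation; its branch on differing velocity and acceleration signs is empty and does not affect the result.
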(fn GetTimeUntilVelocityIsReached
  (params (StartVelocity :type Float%20%28single-precision%29) (EndVelocity :type Float%20%28single-precision%29) (Acceleration :type Float%20%28single-precision%29))
  (LocalVariables|SetV1 StartVelocity)
  (LocalVariables|SetV2 EndVelocity)
  (LocalVariables|SetA Acceleration)
  (if (Math|Boolean|ORBoolean (and (== (LocalVariables|GetA) 0.0) (!= (LocalVariables|GetV1) (LocalVariables|GetV2))) (and (< (LocalVariables|GetA) 0.0) (> (LocalVariables|GetV2) (LocalVariables|GetV1))) (and (> (LocalVariables|GetA) 0.0) (> (LocalVariables|GetV1) (LocalVariables|GetV2))))
    (Development|PrintString 0 "Warning: Velocity is never achieved." false)
    (return 9999999.0)
    (else
      (return (/ (- (LocalVariables|GetV2) (LocalVariables|GetV1)) (LocalVariables|GetA))))))

(fn GetDistanceAfterAcceleration
  (params (StartVelocity :type Float%20%28single-precision%29) (Time :type Float%20%28single-precision%29) (Acceleration :type Float%20%28single-precision%29))
  (LocalVariables|SetV StartVelocity)
  (LocalVariables|SetT Time)
  (LocalVariables|SetA Acceleration)
  (if (!= (Math|Float|Sign(Float) (LocalVariables|GetV)) (Math|Float|Sign(Float) (LocalVariables|GetA)))
    _
    (else
      _))
  (return (+ (* (LocalVariables|GetV) (LocalVariables|Gett)) (* (Math|Float|MakeLiteralFloat 0.5) (LocalVariables|Geta) (Math|Float|Power (LocalVariables|Gett) 2.0)))))