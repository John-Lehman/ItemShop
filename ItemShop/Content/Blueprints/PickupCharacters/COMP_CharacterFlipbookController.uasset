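; Component that drives the Paper2D flipbook animation and left/right facing of its owning PAWN_PickupCharacter.
; Every tick it rotates the flipbook to match the sign of the movement component's X direction.
; When Free, it picks idle, walk or run from velocity thresholds, using Hold variants while carrying an object; all other pickup states use HeldMaintain.
; The flipbook is only reassigned when the target differs from the current one.
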(event EventBeginPlay
  (bind _aspawn_pickup_character (Utilities|Casting|CastToPAWN_PickupCharacter (Components|GetOwner)))
  (Variables|Character|SetPickupCharacter _aspawn_pickup_character)
  (Variables|Character|SetFlipbookComponent (Variables|/Game/Blueprints/PickupCharacters/PAWN_PickupCharacter.PAWN_PickupCharacter_C|GetPaperFlipbook (Variables|Character|GetPickupCharacter))))

(event EventTick
  (params (DeltaSeconds :type Float%20%28single-precision%29))
  (CallFunction|UpdateState))

(fn GetMovementFlipBook
  (params (Velocity :type Float%20%28single-precision%29) (IsHolding :type Boolean))
  (LocalVariables|SetTargetVelocity Velocity)
  (LocalVariables|SetIsHoldingItem IsHolding)
  (if (<= (LocalVariables|GetTargetVelocity) (Variables|VelocityThreshold|GetVelocityThreshold_Walk))
    (return (select (LocalVariables|GetIsHoldingItem) (Variables|FlipbookStates|GetHold_Idle) (Variables|FlipbookStates|GetIdle)))
    (elif (<= (LocalVariables|GetTargetVelocity) (Variables|VelocityThreshold|GetVelocityThreshold_Run))
      (return (select (LocalVariables|GetIsHoldingItem) (Variables|FlipbookStates|GetHold_Walk) (Variables|FlipbookStates|GetWalk)))
      (else
        (return (select (LocalVariables|GetIsHoldingItem) (Variables|FlipbookStates|GetHold_Run) (Variables|FlipbookStates|GetRun)))))))

(fn SetDirection
  (params (Direction :type Vector%202D%20Structure))
  (Variables|StateVariables|SetDirection Direction)
  (if (> (.x (Variables|StateVariables|GetDirection)) 0.0)
    (Transformation|SetRelativeRotation (Variables|Character|GetFlipbookComponent) "180.000000,0.000000,-90.000000" false false)
    (elif (< (.x (Variables|StateVariables|GetDirection)) 0.0)
      (Transformation|SetRelativeRotation (Variables|Character|GetFlipbookComponent) "0.000000,0.000000,-90.000000" false false))))

(fn UpdateState
  (LocalVariables|SetMovementCOMP (Actor|GetComponentbyClass (Variables|Character|GetPickupCharacter) "/Game/Blueprints/PickupCharacters/COMP_CharacterMovement.COMP_CharacterMovement_C"))
  (CallFunction|SetDirection (Default|GetDirection (LocalVariables|GetMovementCOMP)))
  (Utilities|FlowControl|Sequence
    (:then_0
      (bind _state (Default|GetPickupState (Variables|Character|GetPickupCharacter)))
      (switch Utilities|FlowControl|Switch|SwitchonENUM_PickupState _state
        (:NewEnumerator0
          (if (Utilities|IsValid (LocalVariables|GetMovementCOMP))
            (LocalVariables|SetFlipBook_Target (CallFunction|GetMovementFlipBook (Default|GetVelocity (LocalVariables|GetMovementCOMP)) (Utilities|IsValid (Variables|/Game/Blueprints/PickupCharacters/PAWN_PickupCharacter.PAWN_PickupCharacter_C|GetHeldObject (Variables|Character|GetPickupCharacter)))))))
        (:NewEnumerator1
          (LocalVariables|SetFlipBook_Target (Variables|FlipbookStates|GetHeld_Maintain)))
        (:NewEnumerator2
          (LocalVariables|SetFlipBook_Target (Variables|FlipbookStates|GetHeld_Maintain)))
        (:NewEnumerator3
          (LocalVariables|SetFlipBook_Target (Variables|FlipbookStates|GetHeld_Maintain)))
        (:NewEnumerator4
          (LocalVariables|SetFlipBook_Target (Variables|FlipbookStates|GetHeld_Maintain)))))
    (:then_1
      (LocalVariables|SetFlipBook_Current (Class|PaperFlipbookComponent|GetFlipbook (Variables|Character|GetFlipbookComponent)))
      (if (!= (LocalVariables|GetFlipBook_Target) (LocalVariables|GetFlipBook_Current))
        (Sprite|SetFlipbook (Variables|Character|GetFlipbookComponent) (LocalVariables|GetFlipBook_Target))))))